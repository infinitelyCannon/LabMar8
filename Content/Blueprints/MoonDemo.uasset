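; MoonDemo is an actor Blueprint that moves itself every Tick along a path around a Center, apparently as a moon orbit demo.
; A Slerp call computes each position from axis, initial angle, radius, speed, perpendicular and radial offsets, and optional radius clamping.
; An SDelta variable accumulates DeltaSeconds as the elapsed time fed into that call, and the result is applied with SetActorLocation without sweeping.
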(event `self.ReceiveTick`
  (params (DeltaSeconds :type "Float (single-precision)"))
  (bind _sdelta (`self.sDelta`))
  (`self.K2_SetActorLocation` (`.ReturnValue` (`MyTestLib.Slerp` (`self.Center`) (`self.Axis`) (`self.InitialAngle`) _sdelta (`self.Radius`) (`self.Speed`) (`self.PerpendicularOffset`) (`self.RadialOffset`) (`self.MinRadius`) (`self.MaxRadius`) (`self.ClampMovement`))))
  (set `self.sDelta` (+ _sdelta DeltaSeconds)))

(fn `UserConstructionScript`)
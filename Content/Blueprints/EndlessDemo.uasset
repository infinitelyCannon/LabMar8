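; EndlessDemo is a demo actor that spawns three MuhTestCube actors in a row along Y and animates the first.
; Each Tick recomputes a midpoint from the first cube's current location and an offset copy, then moves it with RotateAroundTarget about the X axis.
; A fixed per-frame angle step advances CubeIdx after reaching 180.
; The later stages are empty, so the other two cubes never move.
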(event `self.ReceiveBeginPlay`
  (bind _returnvalue (`|SpawnActorFromClass` "/Game/Blueprints/MuhTestCube.MuhTestCube_C" (`KismetMathLibrary.MakeTransform` (0.0 0.0 0.0)) "Undefined" "OverrideRootScale" null null))
  (set `self.Box1` _returnvalue)
  (bind _returnvalue_2 (`|SpawnActorFromClass` "/Game/Blueprints/MuhTestCube.MuhTestCube_C" (`KismetMathLibrary.MakeTransform` (0.0 100.0 0.0)) "Undefined" "OverrideRootScale" null null))
  (set `self.Box2` _returnvalue_2)
  (bind _returnvalue_3 (`|SpawnActorFromClass` "/Game/Blueprints/MuhTestCube.MuhTestCube_C" (`KismetMathLibrary.MakeTransform` (0.0 200.0 0.0)) "Undefined" "OverrideRootScale" null null))
  (set `self.Box3` _returnvalue_3))

(event `self.ReceiveTick`
  (params (DeltaSeconds :type "Float (single-precision)"))
  (bind _cubeidx (`self.cubeIdx`))
  (bind _box1 (`self.Box1`))
  (bind _delta (`self.delta`))
  (bind _returnvalue (`self.K2_GetActorLocation` _box1))
  (if (== _cubeidx 0)
    (bind _center (`self.Midpoint` _returnvalue (+ _returnvalue 300.0)))
    (`self.K2_SetActorLocation` _box1 (`MyTestLib.RotateAroundTarget` _center (1.0 0.0 0.0) _delta 200.0 20.0) false false)
    (bind _output_get (set `self.delta` (+ _delta 10.0)))
    (if (>= _output_get 180.0)
      (set `self.cubeIdx` 1))
    (elif (== _cubeidx 1)
      _
      (elif (== _cubeidx 2)
        _))))

(fn `Midpoint`
  (params (Start :type "Vector Structure") (End :type "Vector Structure"))
  (returns (Center :type "Vector Structure"))
  (return (/ (+ Start End) 2.0)))

(fn `UserConstructionScript`)
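; SwirlDemo is a demo actor that spawns a stream of MuhTestCube actors set up for a swirling motion.
; Tick accumulates delta time and spawns a cube each time SpawnDelay elapses, until NumSpawned exceeds MaxSpawned.
; Every cube spawns at the same fixed point and receives identical Init settings for center, vertical axis, radius, speed, radial and perpendicular offsets, and clamping.
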(event `self.ReceiveTick`
  (params (DeltaSeconds :type "Float (single-precision)"))
  (bind _mdelta (`self.mDelta`))
  (set `self.mDelta` (+ DeltaSeconds _mdelta))
  (if (and (>= _mdelta (`self.SpawnDelay`)) (<= (`self.NumSpawned`) (`self.MaxSpawned`)))
    (bind _returnvalue (`|SpawnActorFromClass` "/Game/Blueprints/MuhTestCube.MuhTestCube_C" (`KismetMathLibrary.Conv_VectorToTransform` (0.0 0.0 70.0)) "Undefined" "OverrideRootScale" null null))
    (`/Game/Blueprints/MuhTestCube.Init` _returnvalue (0.0 0.0 70.0) (0.0 0.0 1.0) 300.0 15.0 90.0 -15.0 true 0.0 300.0 0.0)
    (set `self.mDelta` 0.0)
    (`/Engine/EditorBlueprintResources/StandardMacros.IncrementInt` (`self.NumSpawned`))))

(fn `UserConstructionScript`)
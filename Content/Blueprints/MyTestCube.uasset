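; A test actor that moves itself from StartPos to EndPos over JourneyTime using spherical interpolation.
; Tick derives an unclamped alpha from the time since BeginPlay and sets the location through Slerp, without sweeping.
; It also computes a midpoint and relative endpoints, but Slerp receives the raw positions.
; Helper functions Test (hand-built dot/acos slerp) and LTest (plain lerp) are not called in the event graph.
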(event `self.ReceiveBeginPlay`
  (set `self.startTime` (`GameplayStatics.GetTimeSeconds`)))

(event `self.ReceiveTick`
  (params (DeltaSeconds :type "Float (single-precision)"))
  (bind _output_get (set `self.center` (* (+ (`self.startPos`) (`self.endPos`)) 0.5)))
  (set `self.relStart` (- (`self.startPos`) _output_get))
  (set `self.relEnd` (- (`self.endPos`) _output_get))
  (bind _output_get_2 (set `self.sDelta` (/ (- (`GameplayStatics.GetTimeSeconds`) (`self.startTime`)) (`self.JourneyTime`))))
  (`self.K2_SetActorLocation` (`MyTestLib.Slerp` (`self.startPos`) (`self.endPos`) _output_get_2)))

(fn `lTest`
  (params (start :type "Vector Structure") (end :type "Vector Structure") (alpha :type "Float (double-precision)"))
  (returns (result :type "Vector Structure"))
  (return (`KismetMathLibrary.VLerp` start end alpha)))

(fn `Test`
  (params (start :type "Vector Structure") (end :type "Vector Structure") (alpha :type "Float (double-precision)"))
  (returns (result :type "Vector Structure"))
  (locals (dot :type "Float (double-precision)") (theta :type "Float (double-precision)") (relVec :type "Vector Structure"))
  (bind _output_get (set `local.dot` (`KismetMathLibrary.FClamp` (`KismetMathLibrary.Dot_VectorVector` start end) -1.0)))
  (bind _output_get_2 (set `local.theta` (* (`KismetMathLibrary.Acos` _output_get) alpha)))
  (bind _output_get_3 (set `local.relVec` (`KismetMathLibrary.Normal` (- end (* start _output_get)))))
  (return (+ (* _output_get_3 (`KismetMathLibrary.Sin` _output_get_2)) (* start (`KismetMathLibrary.Cos` _output_get_2)))))

(fn `UserConstructionScript`)